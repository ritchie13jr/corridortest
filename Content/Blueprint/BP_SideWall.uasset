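; BP_SideWall is a moving wall hazard that respawns the player when touched.
; On BeginPlay it records its location, adds Offset to get the end point, and plays the Movement timeline to lerp the actor between the two without sweeping.
; Overlap of its Box by BP_FirstPersonCharacter calls Respawn on BP_FirstPersonGameMode.
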(event `self.ReceiveBeginPlay`
  (bind _output_get (set `self.StartPos` (`self.K2_GetActorLocation`)))
  (set `self.EndPos` (+ _output_get (`self.Offset`)))
  (bind (_direction _move) (`Timeline|Movement`)
    (:`Update`
      (`self.K2_SetActorLocation` (`KismetMathLibrary.VLerp` (`self.StartPos`) (`self.EndPos`) _move)))))

(event `self.Box.OnComponentBeginOverlap`
  (params (OverlappedComponent :type "PrimitiveComponent Object Reference") (OtherActor :type "Actor Object Reference") (OtherComp :type "PrimitiveComponent Object Reference") (OtherBodyIndex :type Integer) (bFromSweep :type Boolean) (SweepResult :type "HitResult Structure (by ref)"))
  (cast `/Game/FirstPerson/Blueprints/BP_FirstPersonCharacter` OtherActor)
  (bind _asbp_first_person_game_mode (cast `/Game/FirstPerson/Blueprints/BP_FirstPersonGameMode` (`GameplayStatics.GetGameMode`)))
  (`/Game/FirstPerson/Blueprints/BP_FirstPersonGameMode.Respawn` _asbp_first_person_game_mode))

(fn `UserConstructionScript`)